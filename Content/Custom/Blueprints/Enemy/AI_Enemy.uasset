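; Enemy Blueprint that turns to face pawns it sees, takes damage and dies as a ragdoll.
; PawnSensing snaps the actor's rotation toward the seen pawn, with no movement or attack logic.
; A widget component shows normalized health, set on BeginPlay and after each hit.
; Death triggers only on a damage event received with health already depleted, enabling mesh physics and destroying the actor after a delay.
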(event OnSeePawn(PawnSensing)
  (params (Pawn :type Pawn%20Object%20Reference))
  ;[1 1 1] Rotate enemy to character on see it
  (Transformation|SetActorRotation self (Math|Rotator|FindLookatRotation (Transformation|GetActorLocation self) (Transformation|GetActorLocation Pawn))))

(event EventBeginPlay
  ;[1 1 1] Set health value to widget for enemy on spawn it
  (bind _asenemy_health (Utilities|Casting|CastToEnemy_Health (UserInterface|GetWidget (Variables|Default|GetHealth%20widget))))
  (Variables|/Game/Custom/Blueprints/Enemy/Enemy_Health.Enemy_Health_C|SetHealth _asenemy_health (/ (Variables|Default|GetHealth) 1e+02)))

(event Collision|EventActorBeginOverlap
  (params (OtherActor :type Actor%20Object%20Reference)))

(event EventTick
  (params (DeltaSeconds :type Float%20%28single-precision%29)))

(event Game|Damage|EventAnyDamage
  (params (Damage :type Float%20%28single-precision%29) (DamageType :type Damage%20Type%20Object%20Reference) (InstigatedBy :type Controller%20Object%20Reference) (DamageCauser :type Actor%20Object%20Reference))
  ;[1 1 1] Damage and death for this enemy
  (if (> (Variables|Default|GetHealth) 0.0)
    (bind _output_get (Variables|Default|SetHealth (- (Variables|Default|GetHealth) Damage)))
    (bind _asenemy_health (Utilities|Casting|CastToEnemy_Health (UserInterface|GetWidget (Variables|Default|GetHealth%20widget))))
    (Variables|/Game/Custom/Blueprints/Enemy/Enemy_Health.Enemy_Health_C|SetHealth _asenemy_health (/ _output_get 1e+02))
    (else
      (Collision|SetCollisionEnabled (Variables|Character|GetMesh) "PhysicsOnly")
      (Physics|SetSimulatePhysics (Variables|Character|GetMesh) true)
      (Utilities|FlowControl|Delay 6e+01)
      (Actor|DestroyActor))))

(fn ConstructionScript)