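; Master weapon actor that handles firing and reloading for rifle, pistol and sniper, branching on weapon type.
; Shots are hitscan: a short-lived projectile spawns, then impact effect and damage follow at the traced hit after a delay.
; Rifle re-traces from the weapon mesh toward the camera's aim point; pistol and sniper trace from the camera only.
; Shots decrement loaded ammo, empty checks trigger reload, and reloading draws from the character's inventory.
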(event Custom|Custom%20Fire
  (params (Character :type Ana%20Character%20Object%20Reference))
  (bind _inventory_component (Variables|/Game/Custom/Blueprints/Character/Ana_Character.Ana_Character_C|GetInventory_Component Character))
  ;[1 1 1] Fire Function
  (switch Utilities|FlowControl|Switch|SwitchonItem_Type (Variables|Default|GetType)
    (:NewEnumerator2
      (|FireRifle Character (Variables|/Game/Custom/Blueprints/Mains/Inventory/Inventory_Component.Inventory_Component_C|GetRifle%20ammo%20Index _inventory_component)))
    (:NewEnumerator3
      (|FirePistol Character (Variables|/Game/Custom/Blueprints/Mains/Inventory/Inventory_Component.Inventory_Component_C|GetPistol%20ammo%20Index _inventory_component)))
    (:NewEnumerator4
      (|FireSniper Character (Variables|/Game/Custom/Blueprints/Mains/Inventory/Inventory_Component.Inventory_Component_C|GetSniper%20ammo%20Index _inventory_component)))))

(event Custom|Reload
  (params (Character :type Ana%20Character%20Object%20Reference))
  (bind _inventory_component (Variables|/Game/Custom/Blueprints/Character/Ana_Character.Ana_Character_C|GetInventory_Component Character))
  ;[1 1 1] Reload Weapon by it type
  (switch Utilities|FlowControl|Switch|SwitchonItem_Type (Variables|Default|GetType)
    (:NewEnumerator2
      (Utilities|IncreaseAmmo Character (Variables|/Game/Custom/Blueprints/Mains/Inventory/Inventory_Component.Inventory_Component_C|GetRifle%20ammo%20Index _inventory_component) (- (Variables|Default|GetMax%20ammo%20in%20Rifle) (Variables|Default|GetAmmo%20in%20weapon))))
    (:NewEnumerator3
      (Utilities|IncreaseAmmo Character (Variables|/Game/Custom/Blueprints/Mains/Inventory/Inventory_Component.Inventory_Component_C|GetPistol%20ammo%20Index _inventory_component) (- (Variables|Default|GetMax%20ammo%20in%20Pistol) (Variables|Default|GetAmmo%20in%20weapon))))
    (:NewEnumerator4
      (Utilities|IncreaseAmmo Character (Variables|/Game/Custom/Blueprints/Mains/Inventory/Inventory_Component.Inventory_Component_C|GetSniper%20ammo%20Index _inventory_component) (- (Variables|Default|GetMax%20ammo%20in%20Sniper) (Variables|Default|GetAmmo%20in%20weapon)))))
  (Development|PrintString "Reluading" true true "(R=0.000000,G=0.126604,B=1.000000,A=1.000000)"))

(event EventBeginPlay)

(event Collision|EventActorBeginOverlap
  (params (OtherActor :type Actor%20Object%20Reference)))

(fn ConstructionScript)