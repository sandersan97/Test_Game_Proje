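; Player character Blueprint that handles health, HUD, held weapon display and aiming camera placement.
; BeginPlay creates the HUD; AnyDamage updates its health bar and turns on mesh ragdoll physics only for hits arriving at zero health or below.
; Weapon functions show a rifle or pistol mesh based on controller state, or hide it.
; Camera functions snap to aiming points by view type (FPS uses TpsAiming and vice versa) or return to the spring arm.
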(event EventBeginPlay
  ;[1 1 1] Start with full health and create interface HUD
  (bind _output_get (Variables|Default|SetHealth 1e+02))
  (bind _returnvalue (UserInterface|CreateWidget "/Game/Custom/Blueprints/Widgets/HUD.HUD_C" 0 (/ _output_get 1e+02)))
  (bind _output_get_2 (Variables|Default|SetHud%20Reference _returnvalue))
  (UserInterface|Viewport|AddtoViewport _output_get_2 0))

(event Collision|EventActorBeginOverlap
  (params (OtherActor :type Actor%20Object%20Reference)))

(event Game|Damage|EventAnyDamage
  (params (Damage :type Float%20%28single-precision%29) (DamageType :type Damage%20Type%20Object%20Reference) (InstigatedBy :type Controller%20Object%20Reference) (DamageCauser :type Actor%20Object%20Reference))
  (bind _hud_reference (Variables|Default|GetHud%20Reference))
  ;[1 1 1] Damage and death fonksyon
  (if (> (Variables|Default|GetHealth) 0.0)
    (bind _output_get (Variables|Default|SetHealth (- (Variables|Default|GetHealth) Damage)))
    (Variables|/Game/Custom/Blueprints/Widgets/HUD.HUD_C|SetHealth%20Percentes _hud_reference (/ _output_get 1e+02))
    (else
      (Physics|SetSimulatePhysics (Variables|Character|GetMesh) true)
      (Variables|/Game/Custom/Blueprints/Widgets/HUD.HUD_C|SetHealth%20Percentes _hud_reference 0.0))))

(fn ConstructionScript)

(fn AddWeapononHands
  (bind _weapon_mesh (Variables|Default|GetWeapon%20Mesh))
  (bind _asmain_player_controler (Utilities|Casting|CastToMain_Player_Controler (Game|GetPlayerController 0)))
  ;[1 1 1] Get state type for branch is equiped or not
  (if (Utilities|Enum|Equal(Enum) (Variables|/Game/Custom/Blueprints/Mains/Main_Player_Controler.Main_Player_Controler_C|GetCharacter_State _asmain_player_controler) "NewEnumerator4")
    (switch Utilities|FlowControl|Switch|SwitchonItem_Type (.Type (Utilities|Struct|BreakItem_Info (Variables|Default|GetWeapon%20in%20hands)))
      (:NewEnumerator2
        ;[1 1 1] Set weapon static mesh by weapon on hands
        (Transformation|SetRelativeRotation _weapon_mesh "0,90.000000,2.810000" false false)
        (Components|StaticMesh|SetStaticMesh _weapon_mesh "/Game/FPS_Weapon_Bundle/Weapons/Meshes/Ka47/SM_KA47.SM_KA47"))
      (:NewEnumerator3
        (Transformation|SetRelativeRotation _weapon_mesh "0,180.000000,2.810000" false false)
        (Components|StaticMesh|SetStaticMesh _weapon_mesh "/Game/FPS_Weapon_Bundle/Weapons/Meshes/SMG11/SM_SMG11_Nostock_X.SM_SMG11_Nostock_X")))
    (Development|SetHiddeninGame _weapon_mesh false false)
    (else
      (Development|SetHiddeninGame (Variables|Default|GetWeapon%20Mesh) true false))))

(fn RemovefromHands
  (bind _weapon_mesh (Variables|Default|GetWeapon%20Mesh))
  (Components|StaticMesh|SetStaticMesh _weapon_mesh 0)
  (Development|SetHiddeninGame _weapon_mesh true false))

(fn SetCameraAiming
  (bind _camera (Variables|Default|GetCamera))
  (bind _asmain_player_controler (Utilities|Casting|CastToMain_Player_Controler (Game|GetPlayerController 0)))
  (switch Utilities|FlowControl|Switch|SwitchonView_Type (Variables|/Game/Custom/Blueprints/Mains/Main_Player_Controler.Main_Player_Controler_C|GetCamera%20view%20Type _asmain_player_controler)
    (:NewEnumerator0
      (Transformation|SetRelativeLocation _camera (Variables|/Script/Engine.SceneComponent|GetRelativeLocation (Variables|Default|GetTps%20Aiming)) false false))
    (:NewEnumerator1
      (Transformation|SetRelativeLocation _camera (Variables|/Script/Engine.SceneComponent|GetRelativeLocation (Variables|Default|GetFps%20Aiming)) false false))))

(fn ReturnCamera
  (Transformation|SetWorldLocation (Variables|Default|GetCamera) (Transformation|GetSocketLocation (Variables|Default|GetSpringArm) "SpringEndpoint") true false))